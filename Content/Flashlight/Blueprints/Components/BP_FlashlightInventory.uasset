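; Actor component that manages an owner's flashlight inventory: pickup, drop, cycling, equipping, and save/load.
; Name-keyed maps and an ordered stack select the entry that configures the owner's FlashlightComponent, whose battery changes write back into the inventory.
; Interface-fetched meshes, flame and spring arm are re-attached per flashlight, with hand pose and glass material updates.
; State changes mostly replicate through Server-to-Multicast event pairs, and BeginPlay refreshes other owners' active flashlights.
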(event `Server_RefreshInventory`
  ;[0 0 0] Create Components
  (`self.Multi: RefreshInventory`))

(event `Multi: RefreshInventory`
  ;[0 0 0] Create Components
  (bind _outactors (`GameplayStatics.GetAllActorsWithInterface` "/Game/Flashlight/Blueprints/Interfaces/BI_Flashlight.BI_Flashlight_C"))
  (for _array_element _outactors
    (if (!= _array_element (`self.GetOwner`))
      (`KismetSystemLibrary.Delay` 0.2)
      (bind _returnvalue (`Actor.GetComponentByClass` _array_element "BP_FlashlightInventory_C"))
      (if (`/Game/Flashlight/Blueprints/Components/BP_FlashlightInventory.Flashlight Is Active` _returnvalue)
        (`self.Server: Update Flashlight` _returnvalue (`/Game/Flashlight/Blueprints/Components/BP_FlashlightInventory.Equipped Flashlight Name` _returnvalue))
        (`self.MeshVisibilityUpdate`)))))

(event `FlashlightBatteryUpdate`
  ;[0 0 0] Create Components
  (`self.Server: Battery Update`))

(event `FlashlightBatteryDrain`
  ;[0 0 0] Create Components
  (`self.Server: Battery Drain`))

(event `self.ReceiveBeginPlay`
  (bind _returnvalue (`self.GetOwner`))
  (bind _flashlight_component (`self.Flashlight Component`))
  (bind _inventory_stack (`self.Inventory Stack`))
  ;[0 0 0] Create Components
  (bind (_flashlight_skeletal_mesh _flashlight_static_mesh _flame) (message `/Game/Flashlight/Blueprints/Interfaces/BI_Flashlight.Get Flashlight Mesh` (`self.GetOwner`)))
  (`self.SetIsReplicated` _flashlight_skeletal_mesh true)
  (`self.SetIsReplicated` _flashlight_static_mesh true)
  (`self.SetIsReplicated` _flame true)
  (bind (_flashlight_springarm _flashlight_inner_spotlight _flashlight_outer_spotlight _lantern_point_light _flashlight_component_2 _character_mesh) (message `/Game/Flashlight/Blueprints/Interfaces/BI_Flashlight.Get Flashlight Components` _returnvalue))
  (set `self.Flashlight Component` _flashlight_component_2)
  (`/Engine/EditorBlueprintResources/StandardMacros.IsValid` _character_mesh
    (:`Is Valid`
      (set `self.Character Mesh` _character_mesh))
    (:`Is Not Valid`
      (bind _ascharacter (cast `Character` _returnvalue)
        (:`then`
          (set `self.Character Mesh` (`Character.Mesh` _ascharacter)))
        (:`CastFailed`
          _))))
  (`|ExecutionSequence`
    (:`then_1`
      (`KismetSystemLibrary.RetriggerableDelay` 0.3)
      (if (not (< (`KismetArrayLibrary.Array_LastIndex` _inventory_stack) 0))
        (bind _output_get (set `self.Equipped Flashlight Name` (`|GetArrayItem` _inventory_stack)))
        (set `self.Inventory Last Index` 0)
        (set `self.Flashlight Is Equiped` true)
        (`self.Server: Update Flashlight` _output_get)))
    (:`then_2`
      (`KismetSystemLibrary.RetriggerableDelay` 0.31)
      (set `self.Use Idle Hand Pose` (`/Game/Flashlight/Blueprints/Components/BP_Flashlight.Use Idle Hand Pose` (`self.Flashlight Component`)))
      (`self.HandPoseUpdate`))
    (:`then_3`
      (`self.Server_RefreshInventory`))
    (:`then_4`
      (add `/Game/Flashlight/Blueprints/Components/BP_Flashlight.FlashlightBatteryUpdate` _flashlight_component (delegate `FlashlightBatteryUpdate`))
      (add `/Game/Flashlight/Blueprints/Components/BP_Flashlight.FlashlightBatteryDrain` _flashlight_component (delegate `FlashlightBatteryDrain`)))))

(event `Server: Post Pickup`
  (params (`Equipped Flashlight Name` :type String) (Equip :type Boolean))
  ;[0 0 0] Pickup Flashlight
  (`self.Multi: Post Pickup` `Equipped Flashlight Name` Equip))

(event `Multi: Post Pickup`
  (params (`Equipped Flashlight Name` :type String) (Equip :type Boolean))
  ;[0 0 0] Pickup Flashlight
  (if (`self.Flashlight Is Equiped`)
    _
    (elif Equip
      (bind _output_get (set `self.Equipped Flashlight Name` `Equipped Flashlight Name`))
      (set `self.Flashlight Is Equiped` true)
      (set `self.Flashlight Is Active` true)
      (`self.Server: Update Flashlight` _output_get))))

(event `Server: Post Drop`
  (params (`Equipped Flashlight Name` :type String) (`Equip Next?` :type Boolean))
  ;[0 0 0] Drop Flashlight
  (`self.Multi: Post Drop` `Equipped Flashlight Name` `Equip Next?`))

(event `Multi: Post Drop`
  (params (`Equipped Flashlight Name` :type String) (`Equip Next?` :type Boolean))
  (bind _flashlight_component (`self.Flashlight Component`))
  ;[0 0 0] Drop Flashlight
  (if (`/Game/Flashlight/Blueprints/Components/BP_Flashlight.Flashlight On` _flashlight_component)
    (`/Game/Flashlight/Blueprints/Components/BP_Flashlight.Switch Flashlight` _flashlight_component "NewEnumerator0")
    (`self.Server: Switch Flashlight Update`))
  (if (`KismetStringLibrary.EqualEqual_StrStr` `Equipped Flashlight Name` (`self.Equipped Flashlight Name`))
    (set `self.Equipped Flashlight Name` "")
    (set `self.Flashlight Is Equiped` false)
    (set `self.Flashlight Is Active` false)
    (`self.MeshVisibilityUpdate`)
    (if `Equip Next?`
      (`self.NextFlashlight`))))

(event `EquipFlashlight`
  ;[0 0 0] Equip/Unnequip
  (`self.Multi: EquipLight`))

(event `Multi: EquipLight`
  (bind _flashlight_component (`self.Flashlight Component`))
  ;[0 0 0] Equip/Unnequip
  (if (`self.Flashlight Is Equiped`)
    (if (`/Game/Flashlight/Blueprints/Components/BP_Flashlight.Flashlight On` _flashlight_component)
      (`/Game/Flashlight/Blueprints/Components/BP_Flashlight.Switch Flashlight` _flashlight_component "NewEnumerator0")
      (`self.Server: Switch Flashlight Update`)
      (`KismetSystemLibrary.RetriggerableDelay` 0.5))
    (set `self.Flashlight Is Active` (not (`self.Flashlight Is Active`)))
    (`self.HandPoseUpdate`)
    (`self.MeshVisibilityUpdate`)))

(event `Server: Update Flashlight`
  (params (`Flashlight Name` :type String))
  ;[0 0 0] Switch Flashlight
  (`self.Multi: Update Flashlight` `Flashlight Name`))

(event `NextFlashlight`
  ;[0 0 0] Switch Flashlight
  (`self.Server: Next`))

(event `PreviousFlashlight`
  ;[0 0 0] Switch Flashlight
  (`self.Server: Prev`))

(event `Server: Switch Flashlight Update`
  ;[0 0 0] Switch Flashlight
  (`self.Multi: Switch Flashlight Update`))

(event `Multi: Update Flashlight`
  (params (`Flashlight Name` :type String))
  (bind (_value _returnvalue) (`BlueprintMapLibrary.Map_Find` (`self.Flashlight Inventory List`) `Flashlight Name`))
  ;[0 0 0] Switch Flashlight
  (bind _output_get (set `self.Equiped Flashlight Info` _value))
  (set `self.Equiped Flashlight Mesh Info` (`BlueprintMapLibrary.Map_Find` (`self.Available Flashlights Meshes`) `Flashlight Name`))
  (if _returnvalue
    (`/Game/Flashlight/Blueprints/Components/BP_Flashlight.Flashlight Update` (`self.Flashlight Component`) _output_get)
    (bind _output_get_2 (set `self.Use Idle Hand Pose` (`.UseIdleHandPose_47_EEFB883E4FCA5E5CE5683FAF90DE9767` (break `/Game/Flashlight/Blueprints/Structures/SFlashlight` _output_get))))
    (if _output_get_2
      (`self.HandPoseUpdate`))
    (`self.Server: Update Flashlight Mesh`)
    (`|ExecutionSequence`
      (:`then_0`
        (`self.Server: Check Flame Status`))
      (:`then_1`
        (`self.Server: Check Glass`)))))

(event `Multi: Switch Flashlight Update`
  ;[0 0 0] Switch Flashlight
  (`|ExecutionSequence`
    (:`then_0`
      (`self.Server: Check Flame Status`))
    (:`then_1`
      (`self.Server: Check Glass`))))

(event `Server: Next`
  ;[0 0 0] Switch Flashlight
  (`self.Multi: Next`))

(event `Multi: Next`
  (bind _returnvalue (`KismetArrayLibrary.Array_LastIndex` (`self.Inventory Stack`)))
  (bind _returnvalue_2 (+ (`self.Inventory Last Index`) 1))
  ;[0 0 0] Switch Flashlight
  (if (not (< _returnvalue 0))
    (set `self.Inventory Last Index` (`KismetMathLibrary.SelectInt` 0 _returnvalue_2 (> _returnvalue_2 _returnvalue)))
    (for (_array_element _array_index) (`self.Inventory Stack`)
      (if (and (== _array_index (`self.Inventory Last Index`)) (`.Flashlight In Inventory` (`self.Get Flashlight` _array_element)))
        (set `self.Inventory Last Index` _array_index)
        (set `self.Equipped Flashlight Name` _array_element)
        (set `self.Flashlight Is Equiped` true)
        (break))))
  (if (`KismetStringLibrary.EqualEqual_StrStr` (`self.Equipped Flashlight Name`))
    (set `self.Flashlight Is Equiped` false)
    (else
      (`self.Server: Update Flashlight` (`self.Equipped Flashlight Name`)))))

(event `Server: Prev`
  ;[0 0 0] Switch Flashlight
  (`self.Multi: Prev`))

(event `Multi: Prev`
  (bind _returnvalue (`KismetArrayLibrary.Array_LastIndex` (`self.Inventory Stack`)))
  (bind _returnvalue_2 (- (`self.Inventory Last Index`) 1))
  ;[0 0 0] Switch Flashlight
  (if (< _returnvalue 0)
    (if (`KismetStringLibrary.EqualEqual_StrStr` (`self.Equipped Flashlight Name`)) :!label _label
      (set `self.Flashlight Is Equiped` false)
      (else
        (`self.Server: Update Flashlight` (`self.Equipped Flashlight Name`))))
    (else
      (set `self.Inventory Last Index` (`KismetMathLibrary.SelectInt` _returnvalue _returnvalue_2 (< _returnvalue_2 0)))
      (bind (_arrayindex _arrayelement) (`/Engine/EditorBlueprintResources/StandardMacros.ReverseForEachLoop` (`self.Inventory Stack`))
        (:`LoopBody`
          (if (and (== _arrayindex (`self.Inventory Last Index`)) (`.Flashlight In Inventory` (`self.Get Flashlight` _arrayelement)))
            (set `self.Inventory Last Index` _arrayindex)
            (set `self.Equipped Flashlight Name` _arrayelement)
            (set `self.Flashlight Is Equiped` true)))
        (:`Completed`
          (goto _label))))))

(event `Server: Update Flashlight Mesh`
  ;[0 0 0] Spawn Mesh
  (`self.Multi: Update Flashlight Mesh`))

(event `Multi: Update Flashlight Mesh`
  (bind _returnvalue (`self.GetOwner`))
  (bind _returnvalue_2 (`self.GetOwner`))
  (bind (_flashlightskeletalmesh _usestaticmesh_ _flashlightstaticmesh _lightsocket _stablelight _ragdollphysics _charactermeshsocket _charactermeshoffset _lightoffset _useglasslight_ _lightindex _useflame_ _flameoffset) (break `/Game/Flashlight/Blueprints/Structures/SFLMesh` (`self.Equiped Flashlight Mesh Info`)))
  ;[0 0 0] Spawn Mesh
  (bind (_flashlight_skeletal_mesh _flashlight_static_mesh _flame) (message `/Game/Flashlight/Blueprints/Interfaces/BI_Flashlight.Get Flashlight Mesh` _returnvalue_2))
  (`SceneComponent.SetVisibility` _flashlight_skeletal_mesh false false)
  (`SceneComponent.SetVisibility` _flashlight_static_mesh false false)
  (`SceneComponent.SetVisibility` _flame false false)
  (bind _flashlight_springarm (message `/Game/Flashlight/Blueprints/Interfaces/BI_Flashlight.Get Flashlight Components` _returnvalue_2))
  (if _usestaticmesh_
    (`StaticMeshComponent.SetStaticMesh` _flashlight_static_mesh _flashlightstaticmesh)
    (else
      (`SkinnedMeshComponent.SetSkinnedAssetAndUpdate` _flashlight_skeletal_mesh _flashlightskeletalmesh true)
      (for (_array_element _array_index) (`SkeletalMesh.Materials` _flashlightskeletalmesh)
        (`PrimitiveComponent.SetMaterial` _flashlight_skeletal_mesh _array_index (`.MaterialInterface` (break `SkeletalMaterial` _array_element))))))
  (bind _returnvalue_3 (select `bool` _usestaticmesh_ :`false` _flashlight_skeletal_mesh :`true` _flashlight_static_mesh :!type "SceneComponent Object Reference"))
  (`SceneComponent.SetVisibility` _returnvalue_3 (`self.Flashlight Is Active`) false)
  (`SceneComponent.K2_AttachToComponent` _returnvalue_3 (`self.Character Mesh`) _charactermeshsocket "SnapToTarget" "SnapToTarget" "SnapToTarget" true)
  (`SceneComponent.K2_SetRelativeTransform` _returnvalue_3 _charactermeshoffset false true)
  (if _stablelight
    (`SceneComponent.K2_AttachToComponent` _flashlight_springarm (`Character.CapsuleComponent` (cast `Character` (`self.GetOwner`) :!pure true)) "None" "SnapToTarget" "SnapToTarget" "SnapToTarget" true)
    (else
      (`SceneComponent.K2_AttachToComponent` _flashlight_springarm _returnvalue_3 _lightsocket "SnapToTarget" "SnapToTarget" "SnapToTarget" true)))
  (`SceneComponent.K2_SetRelativeTransform` _flashlight_springarm _lightoffset false true)
  (if _useflame_
    (`SceneComponent.K2_AttachToComponent` _flame _returnvalue_3 _lightsocket "SnapToTarget" "SnapToTarget" "SnapToTarget" true)
    (`SceneComponent.K2_SetRelativeTransform` _flame _flameoffset false true)
    (`SceneComponent.SetVisibility` _flame (`self.Flashlight Is Active`) false))
  (if _ragdollphysics
    (bind _flashlight_skeletal_mesh_2 (message `/Game/Flashlight/Blueprints/Interfaces/BI_Flashlight.Get Flashlight Mesh` _returnvalue))
    (`PrimitiveComponent.SetCollisionObjectType` _flashlight_skeletal_mesh_2 "ECC_PhysicsBody")
    (`PrimitiveComponent.SetCollisionEnabled` _flashlight_skeletal_mesh_2 "QueryAndPhysics")
    (set `PrimitiveComponent.CanCharacterStepUpOn` "ECB_Yes" _flashlight_skeletal_mesh_2)
    (`PrimitiveComponent.SetCollisionResponseToChannel` _flashlight_skeletal_mesh_2 "ECC_WorldStatic" "ECR_Ignore")
    (`PrimitiveComponent.SetCollisionResponseToChannel` _flashlight_skeletal_mesh_2 "ECC_WorldDynamic" "ECR_Ignore")
    (`PrimitiveComponent.SetCollisionResponseToChannel` _flashlight_skeletal_mesh_2 "ECC_Pawn" "ECR_Ignore")
    (`PrimitiveComponent.SetCollisionResponseToChannel` _flashlight_skeletal_mesh_2 "ECC_Visibility" "ECR_Ignore")
    (`PrimitiveComponent.SetCollisionResponseToChannel` _flashlight_skeletal_mesh_2 "ECC_Camera" "ECR_Ignore")
    (`PrimitiveComponent.SetCollisionResponseToChannel` _flashlight_skeletal_mesh_2 "ECC_PhysicsBody" "ECR_Ignore")
    (`PrimitiveComponent.SetCollisionResponseToChannel` _flashlight_skeletal_mesh_2 "ECC_Vehicle" "ECR_Ignore")
    (`PrimitiveComponent.SetCollisionResponseToChannel` _flashlight_skeletal_mesh_2 "ECC_Destructible" "ECR_Ignore")
    (else
      (bind _flashlight_skeletal_mesh_3 (message `/Game/Flashlight/Blueprints/Interfaces/BI_Flashlight.Get Flashlight Mesh` _returnvalue))
      (`PrimitiveComponent.SetCollisionEnabled` _flashlight_skeletal_mesh_3 "NoCollision"))))

(event `Server: Check Glass`
  ;[0 0 0] Check Light/Flame
  (`self.Multi: Check Glass`))

(event `Multi: Check Glass`
  (bind _flashlight_component (`self.Flashlight Component`))
  (bind _flashlight_component_2 (`self.Flashlight Component`))
  (bind ((`UseStaticMesh?_31_C779067F48FDE09046039DBAF2F42137` _usestaticmesh_) (`LightIndex_67_1D6DD74741A8D6DAB6D8868A0653B723` _lightindex)) (break `/Game/Flashlight/Blueprints/Structures/SFLMesh` (`self.Equiped Flashlight Mesh Info`)))
  (bind _flashlight_on (`/Game/Flashlight/Blueprints/Components/BP_Flashlight.Flashlight On` _flashlight_component_2))
  ;[0 0 0] Check Light/Flame
  (`KismetSystemLibrary.Delay` (+ (`/Game/Flashlight/Blueprints/Components/BP_Flashlight.Switch Delay` _flashlight_component_2) 0.1))
  (if (and (`|EnumEquality` (`/Game/Flashlight/Blueprints/Components/BP_Flashlight.Flashlight Style` _flashlight_component) "NewEnumerator0") (`.UseGlassLight?_71_0531EC11411E3CA66148AE96A7F34CE0` (break `/Game/Flashlight/Blueprints/Structures/SFLMesh` (`self.Equiped Flashlight Mesh Info`))))
    (bind (_flashlight_skeletal_mesh _flashlight_static_mesh) (message `/Game/Flashlight/Blueprints/Interfaces/BI_Flashlight.Get Flashlight Mesh` (`self.GetOwner`)))
    (bind _returnvalue (select `bool` _usestaticmesh_ :`false` _flashlight_skeletal_mesh :`true` _flashlight_static_mesh :!type "PrimitiveComponent Object Reference"))
    (`PrimitiveComponent.SetMaterial` _returnvalue _lightindex (select `bool` _flashlight_on :`false` "/Game/Flashlight/Materials/MI_FL_Glass.MI_FL_Glass" :`true` "/Game/Flashlight/Materials/MI_FL_GlowingGlass.MI_FL_GlowingGlass" :!type "MaterialInterface Object Reference"))
    (if _flashlight_on
      (bind _returnvalue_2 (`PrimitiveComponent.CreateDynamicMaterialInstance` _returnvalue _lightindex "/Game/Flashlight/Materials/MI_FL_GlowingGlass.MI_FL_GlowingGlass" "None"))
      (`MaterialInstanceDynamic.SetVectorParameterValue` _returnvalue_2 "Glass Light Color" (`/Game/Flashlight/Blueprints/Components/BP_Flashlight.Inner Flashlight Color` _flashlight_component)))))

(event `Server: Check Flame Status`
  ;[0 0 0] Check Light/Flame
  (`self.Multi: Check Flame Status`))

(event `Multi: Check Flame Status`
  (bind _flashlight_component (`self.Flashlight Component`))
  ;[0 0 0] Check Light/Flame
  (`KismetSystemLibrary.Delay` (+ (`/Game/Flashlight/Blueprints/Components/BP_Flashlight.Switch Delay` _flashlight_component) 0.1))
  (if (`|EnumEquality` (`/Game/Flashlight/Blueprints/Components/BP_Flashlight.Flashlight Style` (`self.Flashlight Component`)) "NewEnumerator1")
    (bind (_flashlight_skeletal_mesh _flashlight_static_mesh _flame) (message `/Game/Flashlight/Blueprints/Interfaces/BI_Flashlight.Get Flashlight Mesh` (`self.GetOwner`)))
    (`SceneComponent.SetHiddenInGame` _flame (not (`/Game/Flashlight/Blueprints/Components/BP_Flashlight.Flashlight On` _flashlight_component)) false)))

(event `Server: Battery Drain`
  ;[0 0 0] Battery Update
  (`self.Multi: Battery Drain`))

(event `Server: Battery Update`
  ;[0 0 0] Battery Update
  (`self.Multi: Battery Update`))

(event `Multi: Battery Drain`
  (bind _flashlight_inventory_list (`self.Flashlight Inventory List`))
  (bind _equipped_flashlight_name (`self.Equipped Flashlight Name`))
  (bind (_lighttype _setupspringarm _setupinnerspotlight _setupouterspotlight _setuplanternlight _batterysetup _useaimoffset _useidlehandpose _switchonsoundeffect _switchoffsoundeffect _switchemptybattery _switchonvisualeffect _switchoffvisualeffect _switchdelay _flashlightaimoffset _flashlightaimoffsetpose _flashlighthandpose _uselefthand _blendarmspose _indirectlightdistance _pointlightcastshadow) (break `/Game/Flashlight/Blueprints/Structures/SFlashlight` (`self.Update Flashlight Info`)))
  (bind (_value _returnvalue) (`BlueprintMapLibrary.Map_Find` _flashlight_inventory_list _equipped_flashlight_name))
  (bind (_batteryusage _batterydrainrate _maxbattery _extrabattery _maxextrabattery) (break `/Game/Flashlight/Blueprints/Structures/SFLBattery` _batterysetup))
  ;[0 0 0] Battery Update
  (if _returnvalue
    (set `self.Update Flashlight Info` _value)
    (`BlueprintMapLibrary.Map_Remove` _flashlight_inventory_list _equipped_flashlight_name)
    (`BlueprintMapLibrary.Map_Add` _flashlight_inventory_list _equipped_flashlight_name (make `/Game/Flashlight/Blueprints/Structures/SFlashlight` _lighttype _setupspringarm _setupinnerspotlight _setupouterspotlight _setuplanternlight (make `/Game/Flashlight/Blueprints/Structures/SFLBattery` (`/Game/Flashlight/Blueprints/Components/BP_Flashlight.Battery Usage` (`self.Flashlight Component`)) _batterydrainrate _maxbattery _extrabattery _maxextrabattery) _useaimoffset _useidlehandpose _switchonsoundeffect _switchoffsoundeffect _switchemptybattery _switchonvisualeffect _switchoffvisualeffect _switchdelay _flashlightaimoffset _flashlightaimoffsetpose _flashlighthandpose _uselefthand _blendarmspose _indirectlightdistance _pointlightcastshadow))))

(event `Multi: Battery Update`
  (bind _flashlight_inventory_list (`self.Flashlight Inventory List`))
  (bind _equipped_flashlight_name (`self.Equipped Flashlight Name`))
  (bind (_lighttype _setupspringarm _setupinnerspotlight _setupouterspotlight _setuplanternlight _batterysetup _useaimoffset _useidlehandpose _switchonsoundeffect _switchoffsoundeffect _switchemptybattery _switchonvisualeffect _switchoffvisualeffect _switchdelay _flashlightaimoffset _flashlightaimoffsetpose _flashlighthandpose _uselefthand _blendarmspose _indirectlightdistance _pointlightcastshadow) (break `/Game/Flashlight/Blueprints/Structures/SFlashlight` (`self.Update Flashlight Info`)))
  (bind (_value _returnvalue) (`BlueprintMapLibrary.Map_Find` _flashlight_inventory_list _equipped_flashlight_name))
  (bind (_batteryusage _batterydrainrate _maxbattery _extrabattery _maxextrabattery) (break `/Game/Flashlight/Blueprints/Structures/SFLBattery` _batterysetup))
  ;[0 0 0] Battery Update
  (if _returnvalue
    (set `self.Update Flashlight Info` _value)
    (`BlueprintMapLibrary.Map_Remove` _flashlight_inventory_list _equipped_flashlight_name)
    (`BlueprintMapLibrary.Map_Add` _flashlight_inventory_list _equipped_flashlight_name (make `/Game/Flashlight/Blueprints/Structures/SFlashlight` _lighttype _setupspringarm _setupinnerspotlight _setupouterspotlight _setuplanternlight (make `/Game/Flashlight/Blueprints/Structures/SFLBattery` _batteryusage _batterydrainrate _maxbattery (`/Game/Flashlight/Blueprints/Components/BP_Flashlight.Extra Battery` (`self.Flashlight Component`)) _maxextrabattery) _useaimoffset _useidlehandpose _switchonsoundeffect _switchoffsoundeffect _switchemptybattery _switchonvisualeffect _switchoffvisualeffect _switchdelay _flashlightaimoffset _flashlightaimoffsetpose _flashlighthandpose _uselefthand _blendarmspose _indirectlightdistance _pointlightcastshadow))))

(event `Save Game`
  ;[0 0 0] Save & Load
  (`self.Save`))

(event `Load Game`
  ;[0 0 0] Save & Load
  (bind (_savegame _bsuccess) (`AsyncActionHandleSaveGame.AsyncLoadGameFromSlot` (`self.Slot Name`))
    (:`Completed`
      (if _bsuccess
        (bind _asbp_flashlight_save_game (cast `/Game/Flashlight/Blueprints/SaveGame/BP_FlashlightSaveGame` _savegame))
        (bind _flashlight_inventory (`/Game/Flashlight/Blueprints/SaveGame/BP_FlashlightSaveGame.LoadGame` _asbp_flashlight_save_game))
        (`self.Load` _flashlight_inventory)))))

(event `self.ReceiveTick`
  (params (DeltaSeconds :type "Float (single-precision)")))

(fn `Add Flashlight`
  (params (`Flashlight Name` :type String) (`Equip It?` :type Boolean))
  (bind _flashlight_inventory_list (`self.Flashlight Inventory List`))
  (bind (_value _returnvalue) (`BlueprintMapLibrary.Map_Find` (`self.Available Flashlights`) `Flashlight Name`))
  (if _returnvalue
    (`BlueprintMapLibrary.Map_Remove` _flashlight_inventory_list `Flashlight Name`)
    (`BlueprintMapLibrary.Map_Add` _flashlight_inventory_list `Flashlight Name` _value)
    (`KismetArrayLibrary.Array_AddUnique` (`self.Inventory Stack`) `Flashlight Name`)
    (`self.Server: Post Pickup` `Flashlight Name` `Equip It?`)
    (else
      (`BlueprintMapLibrary.Map_Add` _flashlight_inventory_list `Flashlight Name` _value))))

(fn `Flashlight Is Available?`
  (returns (`Flashlight Is Ready?` :type Boolean))
  (return (`self.Flashlight Is Active`)))

(fn `Get Flashlight`
  (params (`Flashlight Name` :type String))
  (returns (`Flashlight Info` :type "/Game/Flashlight/Blueprints/Structures/SFlashlight Structure") (`Flashlight In Inventory` :type Boolean))
  (bind (_value _returnvalue) (`BlueprintMapLibrary.Map_Find` (`self.Flashlight Inventory List`) `Flashlight Name`))
  (return _value _returnvalue))

(fn `GetEquippedFlashlight`
  (returns (`Equipped Flashlight Name` :type String) (`Is Equipped?` :type Boolean))
  (return (`self.Equipped Flashlight Name`) (`self.Flashlight Is Active`)))

(fn `HandPoseUpdate`
  (bind _flashlight_component (`self.Flashlight Component`))
  (`self.OwnerHasAuthority`
    (:`Server`
      (if (`self.Use Idle Hand Pose`)
        (`/Game/Flashlight/Blueprints/Components/BP_Flashlight.Server: AnimGraphUpdate` _flashlight_component (`/Game/Flashlight/Blueprints/Components/BP_Flashlight.AimOffset` _flashlight_component) (`/Game/Flashlight/Blueprints/Components/BP_Flashlight.AimOffsetPose` _flashlight_component) (select `bool` (`self.Flashlight Is Active`) :`true` (`/Game/Flashlight/Blueprints/Components/BP_Flashlight.HandPose` _flashlight_component)))))))

(fn `Load`
  (params (`Flashlight Inventory List` :type "Map of String to /Game/Flashlight/Blueprints/Structures/SFlashlight Structure"))
  (set `self.Flashlight Inventory List` `Flashlight Inventory List`)
  (`self.Server: Update Flashlight` (`self.Equipped Flashlight Name`)))

(fn `MeshVisibilityUpdate`
  (bind ((`UseStaticMesh?_31_C779067F48FDE09046039DBAF2F42137` _usestaticmesh_) (`UseFlame?_30_F58F272A4C4B211B2A3FFEBA1AA4D3E9` _useflame_)) (break `/Game/Flashlight/Blueprints/Structures/SFLMesh` (`self.Equiped Flashlight Mesh Info`)))
  (bind (_flashlight_skeletal_mesh _flashlight_static_mesh _flame) (message `/Game/Flashlight/Blueprints/Interfaces/BI_Flashlight.Get Flashlight Mesh` (`self.GetOwner`)))
  (`SceneComponent.SetVisibility` (select `bool` _usestaticmesh_ :`false` _flashlight_skeletal_mesh :`true` _flashlight_static_mesh :!type "SceneComponent Object Reference") (`self.Flashlight Is Active`) false)
  (if _useflame_
    (`SceneComponent.SetVisibility` _flame (`self.Flashlight Is Active`) false)))

(fn `Remove Flashlight`
  (params (`Flashlight Name` :type String) (`Equip Next?` :type Boolean))
  (if (`.ReturnValue` (`BlueprintMapLibrary.Map_Find` (`self.Flashlight Inventory List`) `Flashlight Name`))
    (`BlueprintMapLibrary.Map_Remove` (`self.Flashlight Inventory List`) `Flashlight Name`)
    (`KismetArrayLibrary.Array_RemoveItem` (`self.Inventory Stack`) `Flashlight Name`)
    (`self.Server: Post Drop` `Flashlight Name` `Equip Next?`)))

(fn `Save`
  (bind _returnvalue (`GameplayStatics.CreateSaveGameObject` "/Game/Flashlight/Blueprints/SaveGame/BP_FlashlightSaveGame.BP_FlashlightSaveGame_C"))
  (`/Game/Flashlight/Blueprints/SaveGame/BP_FlashlightSaveGame.SaveGame` _returnvalue (`self.Flashlight Inventory List`))
  (bind _output_get (set `self.Slot Name` (`/Game/Flashlight/Blueprints/SaveGame/BP_FlashlightSaveGame.Slot Name` _returnvalue)))
  (`GameplayStatics.SaveGameToSlot` _returnvalue _output_get))

(fn `Unequip Flashlight`
  (set `self.Flashlight Is Equiped` false)
  (set `self.Flashlight Is Active` false))